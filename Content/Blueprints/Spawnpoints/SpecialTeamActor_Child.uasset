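; A child team actor among the spawnpoint Blueprints that tints its Cube mesh with the team color.
; ActivateColor calls ActivateOnServer, which calls ActivateMulticast, a chain named for relaying the change through the server to all clients.
; The final event creates a dynamic material instance from TeamMaterial_Inst on the Cube and sets its Color parameter to TeamColor.
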(event Custom|ActivateOnServer
  (CallFunction|ActivateMulticast))

(event Custom|ActivateMulticast
  (bind _returnvalue (Rendering|Material|CreateDynamicMaterialInstance (Variables|Default|GetCube) 0 "/Game/Blueprints/Spawnpoints/TeamMaterial_Inst.TeamMaterial_Inst" :!class /Script/Engine.PrimitiveComponent))
  (Rendering|Material|SetVectorParameterValue _returnvalue "Color" (Variables|Default|GetTeamColor) :!class /Script/Engine.MaterialInstanceDynamic))

(event EventBeginPlay
  (|CallParentFunction) ; This node is disabled and will not be called.\nDrag off pins to build functionality.
)

(event Collision|EventActorBeginOverlap
  (params (OtherActor :type Actor%20Object%20Reference))
  (|CallParentFunction OtherActor) ; This node is disabled and will not be called.\nDrag off pins to build functionality.
)

(event EventTick
  (params (DeltaSeconds :type Float%20%28single-precision%29))
  (|CallParentFunction DeltaSeconds) ; This node is disabled and will not be called.\nDrag off pins to build functionality.
)

(event EventActivateColor
  (CallFunction|ActivateonServer))

(fn ConstructionScript
  (|CallParentFunction))