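; Player controller for a multiplayer game with a lobby and round-based game modes, linking MyGameMode to each player's UI.
; Events drive the lobby and game widgets: teams, character picks, player lists, scoreboard, countdowns and server messages.
; It tracks kills, deaths and spectating, reporting to the game mode, and routes chat by current mode.
; A status toggle cycles play intent, with an extra take-all-out option on the server.
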(event Custom|AddLobbyWB
  (params (ServerName :type String) (ServerMap :type String) (ServerMode :type String) (ServerSlots :type Integer))
  ;[1 1 1] Create Lobby Widget
  (Variables|Default|SetbShowMouseCursor true)
  (bind _returnvalue (UserInterface|CreateWidget "/Game/Ui/LobbyWB.LobbyWB_C" 0 (Utilities|Text|ToText(String) ServerName) (Utilities|Text|ToText(String) ServerMap) (Utilities|Text|ToText(String) ServerMode) ServerSlots))
  (bind _output_get (Variables|Default|SetLobbyWB _returnvalue))
  (UserInterface|Viewport|AddtoViewport _output_get 1)
  (CallFunction|CreateGameUI))

(event Custom|AddPlayer
  (params (Player :type Text) (PlayerIndex :type Integer) (CharacterImage :type Object%20Object%20Reference) (TeamColor :type Linear%20Color%20Structure))
  ;[1 1 1] Add player to list
  (Default|AddPlayertoList (Variables|Default|GetLobbyWB) Player PlayerIndex CharacterImage TeamColor))

(event Custom|LoadingScreen
  ;[1 1 1] Loading Screen
  (Widget|RemovefromParent (Variables|Default|GetLobbyWB))
  (bind _asmy_game_instance (Utilities|Casting|CastToMyGameInstance (Game|GetGameInstance)))
  (Default|ShowLoadingScreen _asmy_game_instance))

(event Custom|AddGameChatChildToArray
  (params (NewItem :type Game%20Chat%20Message%20Child%20Object%20Reference%20%28by%20ref%29))
  ;[1 1 1] Gamechat
  (Utilities|Array|Add (Variables|Default|GetGameChatArray) NewItem))

(event Custom|toggleStatus
  (bind _returnvalue (Utilities|Text|MakeLiteralText "I want to play"))
  (bind _returnvalue_2 (Utilities|Text|MakeLiteralText "Take all out next round"))
  (bind _returnvalue_3 (Utilities|Text|MakeLiteralText "Let me out"))
  (Networking|SwitchHasAuthority
    (:Authority
      (Utilities|FlowControl|MultiGate false true -1 :!label _label
        (:Out%200
          (Rendering|Components|TextRender|SetText (Variables|/Game/Ui/Game/GameUI.GameUI_C|Getstatus (Variables|Default|GetGameUIWB)) _returnvalue_3 :!label _label_2)
          (Rendering|Components|TextRender|SetText (Variables|/Game/Ui/LobbyWB.LobbyWB_C|Getstatus (Variables|Default|GetLobbyWB)) _returnvalue_3)
          (CallFunction|SetIwanttoPlay false)
          (Networking|SwitchHasAuthority :!label _label_3
            (:Authority
              (CallFunction|AddAllPlayerstoLastRoundPC false))
            (:Remote
              _))
          (CallFunction|CheckEnoughPlayersWhoWanttoPlayPC))
        (:Out%201
          (bind _asmy_game_mode (Utilities|Casting|CastToMyGameMode (Game|GetGameMode)))
          (if (!= (Variables|/Game/Blueprints/MyGameMode.MyGameMode_C|GetGameMode _asmy_game_mode) 0)
            (Rendering|Components|TextRender|SetText (Variables|/Game/Ui/Game/GameUI.GameUI_C|Getstatus (Variables|Default|GetGameUIWB)) _returnvalue_2)
            (Rendering|Components|TextRender|SetText (Variables|/Game/Ui/LobbyWB.LobbyWB_C|Getstatus (Variables|Default|GetLobbyWB)) _returnvalue_2)
            (CallFunction|AddAllPlayerstoLastRoundPC true)
            (else
              (goto _label))))
        (:Out%202
          (Rendering|Components|TextRender|SetText (Variables|/Game/Ui/Game/GameUI.GameUI_C|Getstatus (Variables|Default|GetGameUIWB)) _returnvalue :!label _label_4)
          (Rendering|Components|TextRender|SetText (Variables|/Game/Ui/LobbyWB.LobbyWB_C|Getstatus (Variables|Default|GetLobbyWB)) _returnvalue)
          (CallFunction|SetIwanttoPlay true)
          (goto _label_3))))
    (:Remote
      (Utilities|FlowControl|FlipFlop
        (:A
          (goto _label_2))
        (:B
          (goto _label_4))))))

(event Custom|AddMessageToChat
  (params (NewParam :type Chat%20Message%20Structure%20Structure))
  (bind _lobbywb (Variables|Default|GetLobbyWB))
  ;[1 1 1] LobbyChat
  (if (== (Variables|Default|GetGM) 0)
    (Utilities|IsValid _lobbywb
      (:Is%20Valid
        (Default|AddChildtoChat (Variables|/Game/Ui/LobbyWB.LobbyWB_C|GetChatWindow_0 _lobbywb) NewParam)))
    (else
      (Default|AddChildtoChat (Variables|/Game/Ui/Game/GameUI.GameUI_C|GetGameChatWindow (Variables|Default|GetGameUIWB)) NewParam self))))

(event Custom|HideLoadingScreen
  ;[1 0.6939 0] SetUpPlayerForNewGameMode
  (bind _asmy_game_instance (Utilities|Casting|CastToMyGameInstance (Game|GetGameInstance)))
  (Default|HideLoadingScreen _asmy_game_instance))

(event Custom|AddTeams
  (params (NewParam :type Array%20of%20Teams%20Structur%20Structures))
  (for (_array_element _array_index) NewParam
    (bind _returnvalue (UserInterface|CreateWidget "/Game/Ui/TeamJoinButton.TeamJoinButton_C" 0 (+ _array_index 1) 0 _array_element))
    (Widget|Panel|AddChild (Variables|/Game/Ui/LobbyWB.LobbyWB_C|GetTeamsBox (Variables|Default|GetLobbyWB)) _returnvalue)))

(event Custom|SendImportantServerMessage
  (params (Message :type Text) (delay :type Float%20%28single-precision%29) (Color :type Linear%20Color%20Structure) (Size :type Integer))
  (bind _gameuiwb (Variables|Default|GetGameUIWB))
  (bind _importantservermessagebox (Variables|/Game/Ui/Game/GameUI.GameUI_C|GetImportantServerMessageBox _gameuiwb))
  (bind _box (Variables|/Game/Ui/Game/ImportantServerMessageBox.ImportantServerMessageBox_C|GetBox _importantservermessagebox))
  (bind _returnvalue (UserInterface|CreateWidget "/Game/Ui/Game/ImportantServerMessage.ImportantServerMessage_C" 0 Message delay Color Size))
  (Widget|Panel|AddChild _box _returnvalue)
  (Utilities|FlowControl|Delay delay)
  (Class|PanelWidget|RemoveChild _box _returnvalue))

(event Custom|UpdateServerFromPC
  (bind _asmy_game_mode (Utilities|Casting|CastToMyGameMode (Game|GetGameMode)))
  (Default|UpdateServer _asmy_game_mode))

(event Custom|SetTeamForLobbyWB
  (params (Team :type Integer) (Same? :type Boolean))
  (Variables|/Game/Ui/LobbyWB.LobbyWB_C|SetTeam (Variables|Default|GetLobbyWB) (Math|Integer|SelectInt 0 Team Same?)))

(event Custom|UpdateNumberOfPlayersInEachTeam
  (params (NewParam :type Array%20of%20Integers))
  (for (_array_element _array_index) NewParam
    (bind _asteam_join_button (Utilities|Casting|CastToTeamJoinButton (Class|PanelWidget|GetChildat (Variables|/Game/Ui/LobbyWB.LobbyWB_C|GetTeamsBox (Variables|Default|GetLobbyWB)) _array_index)))
    (Default|UpdateNumberOfPlayers _asteam_join_button _array_element)))

(event Custom|HideRightCountdown
  (Default|HideCountdownRight (Variables|/Game/Ui/Game/GameUI.GameUI_C|GetcountdownRight (Variables|Default|GetGameUIWB))))

(event Custom|HideChat
  ;[1 1 1] Gamechat
  (Variables|Default|SetisChatOpen? false)
  (Input|SetInputModeGameOnly self)
  (Variables|Default|SetbShowMouseCursor false)
  (for _array_element (Variables|Default|GetGameChatArray)
    (Default|ChatOpened _array_element false)))

(event Custom|SelectCharacterOnServer
  (params (Same? :type Boolean) (Selection :type Integer) (SelectedCharacterClass :type Pawn%20Class%20Reference))
  (CallFunction|SelectCharacterMulticast Same? Selection SelectedCharacterClass))

(event Custom|ResetTeamPlayersForUpdate
  (bind _lobbywb (Variables|Default|GetLobbyWB))
  (bind _teamsbox (Variables|/Game/Ui/LobbyWB.LobbyWB_C|GetTeamsBox _lobbywb))
  (for _index (range 0 (Class|PanelWidget|GetChildrenCount _teamsbox))
    (bind _asteam_join_button (Utilities|Casting|CastToTeamJoinButton (Class|PanelWidget|GetChildat _teamsbox _index)))
    (Variables|/Game/Ui/TeamJoinButton.TeamJoinButton_C|SetCurrentPlayersInTeam _asteam_join_button 0)))

(event Custom|SetGameMode
  (params (GameMode :type Integer))
  ;[1 0.6939 0] SetUpPlayerForNewGameMode
  (Variables|Default|SetGameMode GameMode))

(event Custom|SelectCharacterMulticast
  (params (Same? :type Boolean) (SelectedCharacterNumber :type Integer) (SelectedCharacterClass :type Pawn%20Class%20Reference))
  (if Same?
    (Variables|Default|SetSelectedCharacterNumber 0)
    (Variables|Default|SetSelectedCharacterClass 0)
    (else
      (Variables|Default|SetSelectedCharacterNumber SelectedCharacterNumber)
      (Variables|Default|SetSelectedCharacterClass SelectedCharacterClass))))

(event Custom|JoinOrLeaveTeamMulticast
  (params (Team :type Integer) (Same :type Boolean))
  (Variables|Default|SetSelectedTeamNumber (Math|Integer|SelectInt 0 Team Same))
  (Variables|Default|SetSelectedCharacterClass 0)
  (Variables|Default|SetSelectedCharacterNumber 0))

(event Custom|SetDead
  (params (isDead? :type Boolean))
  (bind _output_get (Variables|Default|SetisDead? isDead?))
  (if _output_get
    (Utilities|FlowControl|Delay 0.2)
    (bind _asmy_game_mode (Utilities|Casting|CastToMyGameMode (Game|GetGameMode)))
    (Default|CountLivingPlayers _asmy_game_mode self)))

(event Custom|StartIngameTimer
  (params (Minutes :type Integer) (Seconds :type Integer) (CountUp? :type Boolean))
  (Default|StartCountDown (Variables|/Game/Ui/Game/GameUI.GameUI_C|GetcountdownRight (Variables|Default|GetGameUIWB)) Minutes Seconds CountUp?))

(event Custom|ClearPlayerList
  ;[1 1 1] Clear player list
  (Default|ClearPlayerList (Variables|Default|GetLobbyWB)))

(event Custom|SetTeam_forLobbyWB
  (params (Team :type Integer) (Same :type Boolean))
  (Variables|/Game/Ui/LobbyWB.LobbyWB_C|SetTeam (Variables|Default|GetLobbyWB) (Math|Integer|SelectInt 0 Team Same)))

(event Custom|UpdateAvailableCharactersNoTeams
  (params (NewParam :type Array%20of%20Booleans))
  (for (_array_element _array_index) NewParam
    (bind _ascharacter_button (Utilities|Casting|CastToCharacterButton (Class|PanelWidget|GetChildat (Variables|/Game/Ui/LobbyWB.LobbyWB_C|GetCharacterBox1 (Variables|Default|GetLobbyWB)) _array_index)))
    (Default|ToggleEnabled _ascharacter_button _array_element)))

(event Custom|SetSpectating
  (params (spectate? :type Boolean))
  (Variables|Default|SetSpectating spectate?))

(event Custom|AddMessageFromServerToEachPlayer
  (params (Message :type String) (Color :type Slate%20Color%20Structure) (isServerMessage :type Boolean))
  (bind _self self)
  (bind _playername (Class|AdvancedSessionsLibrary|GetPlayerName _self))
  (bind _chatmessagestructure (Utilities|Struct|MakeChatMessageStructure _playername Message Color isServerMessage))
  ;[1 1 1] LobbyChat
  (bind _asmy_game_mode (Utilities|Casting|CastToMyGameMode (Game|GetGameMode)))
  (for _array_element (Variables|/Game/Blueprints/MyGameMode.MyGameMode_C|GetAllPCs _asmy_game_mode)
    (bind _asmy_player_controller (Utilities|Casting|CastToMyPlayerController _array_element))
    (CallFunction|AddMessagetoChat _asmy_player_controller _chatmessagestructure))
  (bind _asmy_game_mode_2 (Utilities|Casting|CastToMyGameMode (Game|GetGameMode)))
  (Default|AddMessagetoChatHistory _asmy_game_mode_2 _chatmessagestructure))

(event Custom|JoinOrLeaveTeamServer
  (params (Team :type Integer) (Same? :type Boolean))
  (CallFunction|JoinorLeaveTeamMulticast Team Same?))

(event Custom|PlayerDataSetup
  ;[1 1 1] Setup Player Data
  (bind _asmy_game_instance (Utilities|Casting|CastToMyGameInstance (Game|GetGameInstance)))
  (bind _output_get (Variables|Default|SetLan_Name (Variables|/Game/Blueprints/MyGameInstance.MyGameInstance_C|GetLan_Name _asmy_game_instance)))
  (CallFunction|PlayerDataSetuponServer _output_get))

(event Custom|Kick
  (params (Kickindex :type Integer))
  ;[1 1 1] kick player
  (switch int Kickindex
    (:0
      (Game|OpenLevel(byName) "kicked")
      (|DestroySession self))
    (:1
      (Game|OpenLevel(byName) "ServerFull")
      (|DestroySession self))))

(event Custom|StartCountdownCenter
  (params (Minutes :type Integer) (Seconds :type Integer) (DisableMovement? :type Boolean))
  (Utilities|FlowControl|Delay 0.2)
  (Default|StartCountDown (Variables|/Game/Ui/Game/GameUI.GameUI_C|GetcountdownCenter (Variables|Default|GetGameUIWB)) Minutes Seconds)
  (if DisableMovement?
    (bind _asmain_character (Utilities|Casting|CastToMainCharacter (Game|GetPlayerCharacter 0)))
    (Variables|/Game/ThirdPersonBP/Blueprints/MainCharacter.MainCharacter_C|SetWaitingForStart? _asmain_character true)
    (Utilities|FlowControl|Delay (Math|Conversions|ToFloat(Integer) (+ (* Minutes 60) Seconds)))
    (Variables|/Game/ThirdPersonBP/Blueprints/MainCharacter.MainCharacter_C|SetWaitingForStart? _asmain_character false)))

(event Custom|AddKill
  ;[1 1 1] ScoreBoard
  (Math|Integer|IncrementInt (Variables|Default|GetKills)
    (:%20%20
      (if (== (Variables|Default|GetDeaths) 0)
        (Variables|Default|SetKD (Math|Conversions|ToFloat(Integer) (Variables|Default|GetKills)))
        (else
          (Variables|Default|SetKD (/ (Math|Conversions|ToFloat(Integer) (Variables|Default|GetKills)) (Math|Conversions|ToFloat(Integer) (Variables|Default|GetDeaths))))))
      (bind _asmy_game_mode (Utilities|Casting|CastToMyGameMode (Game|GetGameMode)))
      (Default|UpdateScoreBoard _asmy_game_mode))))

(event Custom|ClearScoreBoard
  ;[1 1 1] ScoreBoard
  (Default|Clear (Variables|/Game/Ui/Game/GameUI.GameUI_C|GetScoreBoard (Variables|Default|GetGameUIWB))))

(event Custom|PlayerDataSetupOnServer
  (params (Lan_Name :type String))
  ;[1 1 1] Setup Player Data
  (bind _output_get (Variables|Default|SetLan_Name Lan_Name))
  (Class|AdvancedSessionsLibrary|SetPlayerName self (select (Class|AdvancedSessionsLibrary|HasOnlineSubsystem "STEAM") (Class|AdvancedSessionsLibrary|GetPlayerName self) _output_get))
  (CallFunction|SetUpFinished))

(event Custom|TeleportOnOwningClient
  (params (NewLocation :type Vector))
  (Default|TeleportPlayeronServer (Variables|Default|GetMainCharacterRef) NewLocation))

(event Custom|AddDeath
  ;[1 1 1] ScoreBoard
  (Math|Integer|IncrementInt (Variables|Default|GetDeaths)
    (:%20%20
      (Variables|Default|SetKD (/ (Math|Conversions|ToFloat(Integer) (Variables|Default|GetKills)) (Math|Conversions|ToFloat(Integer) (Variables|Default|GetDeaths))))
      (bind _asmy_game_mode (Utilities|Casting|CastToMyGameMode (Game|GetGameMode)))
      (Default|UpdateScoreBoard _asmy_game_mode))))

(event Custom|SetIwantToPlay
  (params (yes? :type Boolean))
  (Variables|Default|SetIWantToPlay yes?))

(event Custom|AddPlayerToScoreBoard
  (params (Name :type String) (Kills :type Integer) (Deaths :type Integer) (position :type Integer) (KD :type Float%20%28single-precision%29) (isOwnPlayer? :type Boolean) (isNotinTopList? :type Boolean))
  ;[1 1 1] ScoreBoard
  (Default|AddPlayer (Variables|/Game/Ui/Game/GameUI.GameUI_C|GetScoreBoard (Variables|Default|GetGameUIWB)) Name Kills Deaths position KD isOwnPlayer? isNotinTopList?))

(event Custom|SetServerData
  (params (ServerName :type String) (ServerMode :type String))
  ;[1 1 1] ScoreBoard
  (Default|SetServerData (Variables|/Game/Ui/Game/GameUI.GameUI_C|GetScoreBoard (Variables|Default|GetGameUIWB)) ServerName ServerMode))

(event Custom|ShowSpectateButton
  (params (show? :type Boolean))
  (bind _lobbywb (Variables|Default|GetLobbyWB))
  (bind _spectatebutton (Variables|/Game/Ui/LobbyWB.LobbyWB_C|GetspectateButton _lobbywb))
  (if show?
    (Widget|SetVisibility _spectatebutton "Visible")
    (else
      (Widget|SetVisibility _spectatebutton "Collapsed"))))

(event Custom|UpdateAvailableCharactersTeams
  (params (charsInTeam1 :type Array%20of%20Booleans) (charsInTeam2 :type Array%20of%20Booleans) (charsInTeam3 :type Array%20of%20Booleans))
  (for (_array_element _array_index) charsInTeam1
    (bind _ascharacter_button (Utilities|Casting|CastToCharacterButton (Class|PanelWidget|GetChildat (Variables|/Game/Ui/LobbyWB.LobbyWB_C|GetCharacterBox1 (Variables|Default|GetLobbyWB)) _array_index)))
    (Default|ToggleEnabled _ascharacter_button _array_element))
  (for (_array_element_2 _array_index_2) charsInTeam2
    (bind _ascharacter_button_2 (Utilities|Casting|CastToCharacterButton (Class|PanelWidget|GetChildat (Variables|/Game/Ui/LobbyWB.LobbyWB_C|GetCharacterBox2 (Variables|Default|GetLobbyWB)) _array_index_2)))
    (Default|ToggleEnabled _ascharacter_button_2 _array_element_2))
  (for (_array_element_3 _array_index_3) charsInTeam3
    (bind _ascharacter_button_3 (Utilities|Casting|CastToCharacterButton (Class|PanelWidget|GetChildat (Variables|/Game/Ui/LobbyWB.LobbyWB_C|GetCharacterBox3 (Variables|Default|GetLobbyWB)) _array_index_3)))
    (Default|ToggleEnabled _ascharacter_button_3 _array_element_3)))

(event Custom|UpdateNumberOfPlayers
  (params (currentPlayers :type Integer))
  ;[1 1 1] Update Player-Number
  (Variables|/Game/Ui/LobbyWB.LobbyWB_C|SetcurrentPlayers (Variables|Default|GetLobbyWB) currentPlayers))

(event Custom|AddAllPlayersToLastRoundPC
  (params (LastRoundForAllPlayers? :type Boolean))
  (bind _asmy_game_mode (Utilities|Casting|CastToMyGameMode (Game|GetGameMode)))
  (Default|SetAllPlayerstoLastRound _asmy_game_mode LastRoundForAllPlayers?))

(event Custom|CreateGameUI
  ;[1 0.6939 0] SetUpPlayerForNewGameMode
  (Utilities|IsValid (Variables|Default|GetGameUIWB)
    (:Is%20Valid
      (Widget|RemovefromParent (Variables|Default|GetGameUIWB)))
    (:Is%20Not%20Valid
      _))
  (bind _returnvalue (UserInterface|CreateWidget "/Game/Ui/Game/GameUI.GameUI_C"))
  (bind _output_get (Variables|Default|SetGameUIWB _returnvalue))
  (UserInterface|Viewport|AddtoViewport _output_get 0))

(event Custom|SetUpNewGamemodeAndUI
  (params (GM :type Integer) (LoadingScreenTime :type Float%20%28single-precision%29))
  (bind _lobbywb (Variables|Default|GetLobbyWB))
  ;[1 1 1] SetUp Players for Gameplay
  (bind _output_get (Variables|Default|SetGM GM))
  (if (!= _output_get 0)
    (Default|ShowLoadingAnimation (Variables|Default|GetLobbyWB))
    (Utilities|FlowControl|Delay LoadingScreenTime)
    (Widget|SetVisibility (Variables|Default|GetLobbyWB) "Collapsed")
    (Input|SetInputModeGameOnly self)
    (Variables|Default|SetbShowMouseCursor false)
    (else
      (Widget|SetVisibility _lobbywb "Visible")
      (Default|ShowLobbyWB _lobbywb)
      (Input|SetInputModeUIOnly self _lobbywb "DoNotLock")
      (Variables|Default|SetbShowMouseCursor true)
      (if (Networking|IsServer)
        (CallFunction|ToggleStatus)
        (CallFunction|ToggleStatus)))))

(event Custom|SetUpFinished
  ;[1 1 1] Setup Player Data
  (bind _asmy_game_mode (Utilities|Casting|CastToMyGameMode (Game|GetGameMode)))
  (Default|Continue _asmy_game_mode))

(event Custom|CheckEnoughPlayersWhoWantToPlayPC
  (bind _asmy_game_mode (Utilities|Casting|CastToMyGameMode (Game|GetGameMode)))
  (Default|CheckEnoughPlayersWhoWanttoPlay _asmy_game_mode))

(event EventBeginPlay
  ;[1 1 1] Event BeginPlay
  (bind _asmain_character (Utilities|Casting|CastToMainCharacter (Game|GetPlayerCharacter 0)))
  (Variables|Default|SetMainCharacterRef _asmain_character))

(event Input|KeyboardEvents|Enter
  (params (Key :type Key%20Structure))
  (bind _gameuiwb (Variables|Default|GetGameUIWB))
  (bind _gamechatwindow (Variables|/Game/Ui/Game/GameUI.GameUI_C|GetGameChatWindow _gameuiwb))
  ;[1 1 1] Gamechat
  (:Pressed
    (if (not (== (Variables|Default|GetGM) 0))
      (if (not (Variables|Default|GetisChatOpen?))
        (Variables|Default|SetisChatOpen? true)
        (Input|SetInputModeUIOnly self 0 "DoNotLock")
        (Variables|Default|SetbShowMouseCursor true)
        (Widget|SetKeyboardFocus (Variables|/Game/Ui/Game/GameChatWindow.GameChatWindow_C|GetEditableTextBox_0 _gamechatwindow))
        (for _array_element (Variables|Default|GetGameChatArray)
          (Default|ChatOpened _array_element true))
        (Class|ScrollBox|ScrolltoEnd (Variables|/Game/Ui/Game/GameChatWindow.GameChatWindow_C|GetScrollBox_0 _gamechatwindow))))))

(event Input|KeyboardEvents|H
  (params (Key :type Key%20Structure))
  (bind _lobbywb (Variables|Default|GetLobbyWB))
  (:Pressed
    (if (Variables|Default|GetSpectating)
      (Widget|SetVisibility _lobbywb "Visible")
      (Default|ShowLobbyWB _lobbywb)
      (Input|SetInputModeUIOnly self 0 "DoNotLock")
      (Variables|Default|SetbShowMouseCursor true))))

(event Input|KeyboardEvents|L
  (params (Key :type Key%20Structure))
  (:Pressed
    (CallFunction|ToggleStatus)))

(event Input|KeyboardEvents|Tab
  (params (Key :type Key%20Structure))
  (bind _gameuiwb (Variables|Default|GetGameUIWB))
  (bind _scoreboard (Variables|/Game/Ui/Game/GameUI.GameUI_C|GetScoreBoard _gameuiwb))
  ;[1 1 1] ScoreBoard
  (:Pressed
    (Widget|SetVisibility _scoreboard "SelfHitTestInvisible"))
  (:Released
    (Widget|SetVisibility _scoreboard "Collapsed")))

(fn ConstructionScript)