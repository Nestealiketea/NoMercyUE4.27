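; Player-flown F15 jet with simple arcade flight: throttle, yaw, pitch and roll input, without physics simulation.
; Each Tick moves it forward with sweep, easing speed down by Drag when throttle drops and adding gravity as speed falls below MinTrustToNotFall.
; Smoothed axis inputs rotate the jet and deflect rudders, elevators and ailerons.
; Niagara thrusters spawn on BeginPlay, but their throttle-driven update is unwired; debug values print every frame.
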(event EventBeginPlay
  (bind _output_get (Variables|DinamicVariables|SetTrustSpeed (Variables|Constansts|GetMinTrustToNotFall)))
  (Variables|DinamicVariables|SetCurrentSpeed _output_get)
  (bind _returnvalue (Niagara|SpawnSystemAttached "/Game/Test_Content/F15/FX/ThrusterEmitter_System.ThrusterEmitter_System" (Variables|Default|GetFuselage) "ThrusterL" "0, 0, 0" "0, 0, 0" "SnapToTargetIncludingScale" false))
  (Variables|Default|SetThruster_Left_FXS _returnvalue)
  (bind _returnvalue_2 (Niagara|SpawnSystemAttached "/Game/Test_Content/F15/FX/ThrusterEmitter_System.ThrusterEmitter_System" (Variables|Default|GetFuselage) "ThrusterR" "0, 0, 0" "0, 0, 0" "SnapToTargetIncludingScale" false))
  (Variables|Default|SetThruster_Right_FXS _returnvalue_2))

(event EventTick
  (params (DeltaSeconds :type Float%20%28single-precision%29))
  (Private|UpdatePosition DeltaSeconds)
  (Private|PrintVariebles))

(event Input|AxisEvents|InputAxisTrust
  (params (AxisValue :type Float%20%28single-precision%29))
  (Variables|DinamicVariables|SetTrustSpeed (Math|Float|Clamp(Float) (+ (* AxisValue (Utilities|Time|GetWorldDeltaSeconds) (Variables|Constansts|GetTrustMultiplayer)) (Variables|DinamicVariables|GetTrustSpeed)) 0.0 (Variables|Constansts|GetMaxTrustSpeed))))

(event Input|AxisEvents|InputAxisYaw
  (params (AxisValue :type Float%20%28single-precision%29))
  (Private|UpdateYaw (Utilities|Time|GetWorldDeltaSeconds) AxisValue))

(event Input|AxisEvents|InputAxisPitch
  (params (AxisValue :type Float%20%28single-precision%29))
  (Private|UpdatePitch (Utilities|Time|GetWorldDeltaSeconds) AxisValue))

(event Input|AxisEvents|InputAxisRoll
  (params (AxisValue :type Float%20%28single-precision%29))
  (Private|UpdateRoll (Utilities|Time|GetWorldDeltaSeconds) AxisValue))

(event Input|KeyboardEvents|1
  (params (Key :type Key%20Structure :default "None")))

(event Input|KeyboardEvents|2
  (params (Key :type Key%20Structure :default "None")))

(event Input|KeyboardEvents|3
  (params (Key :type Key%20Structure :default "None")))

(event Input|KeyboardEvents|4
  (params (Key :type Key%20Structure :default "None")))

(fn ConstructionScript)

(fn UpdatePosition
  (params (DeltaSeconds :type Float%20%28single-precision%29))
  (Variables|DinamicVariables|SetCurrentSpeed (select (< (Variables|DinamicVariables|GetTrustSpeed) (Variables|DinamicVariables|GetCurrentSpeed)) (Math|Interpolation|FInterpTo (Variables|DinamicVariables|GetCurrentSpeed) (Variables|DinamicVariables|GetTrustSpeed) DeltaSeconds (Variables|Constansts|GetDrag)) (Variables|DinamicVariables|GetTrustSpeed)))
  (LocalVariables|SetNewPositon (* (Transformation|GetActorForwardVector) (* (Variables|DinamicVariables|GetCurrentSpeed) DeltaSeconds)))
  (Variables|DinamicVariables|SetApplyedGravity (Math|Float|MapRangeClamped (Variables|DinamicVariables|GetCurrentSpeed) 0.0 (Variables|Constansts|GetMinTrustToNotFall) (Variables|Constansts|GetGravity) 0.0))
  (Transformation|AddActorWorldOffset (Math|Vector|MakeVector (.X (Math|Vector|BreakVector (LocalVariables|GetNewPositon))) (.Y (Math|Vector|BreakVector (LocalVariables|GetNewPositon))) (- (.Z (Math|Vector|BreakVector (LocalVariables|GetNewPositon))) (* (Variables|DinamicVariables|GetApplyedGravity) DeltaSeconds))) true))

(fn UpdateYaw
  (params (DeltaSeconds :type Float%20%28single-precision%29) (Yaw :type Float%20%28single-precision%29))
  (Variables|DinamicVariables|Rotation|SetTargetYaw Yaw)
  (bind _output_get (Variables|DinamicVariables|Rotation|SetCurrentYaw (Math|Interpolation|FInterpTo (Variables|DinamicVariables|Rotation|GetCurrentYaw) (Variables|DinamicVariables|Rotation|GetTargetYaw) DeltaSeconds 1e+01)))
  (Transformation|AddActorLocalRotation (Math|Rotator|MakeRotator 0.0 0.0 (* _output_get DeltaSeconds 15.0)) false false)
  (Transformation|SetRelativeRotation (Variables|Default|GetSM_rudderR) (Math|Rotator|MakeRotator 0.0 0.0 (Math|Float|MapRangeClamped (Variables|DinamicVariables|Rotation|GetCurrentYaw) -1.0 1.0 (Variables|Constansts|Controller|GetMaxRudderYaw) (Utilities|NegateFloat (Variables|Constansts|Controller|GetMaxRudderYaw)))) false false)
  (Transformation|SetRelativeRotation (Variables|Default|GetSM_rudderL) (Math|Rotator|MakeRotator 0.0 0.0 (Math|Float|MapRangeClamped (Variables|DinamicVariables|Rotation|GetCurrentYaw) -1.0 1.0 (Variables|Constansts|Controller|GetMaxRudderYaw) (Utilities|NegateFloat (Variables|Constansts|Controller|GetMaxRudderYaw)))) false false))

(fn UpdatePitch
  (params (DeltaSeconds :type Float%20%28single-precision%29) (Pitch :type Float%20%28single-precision%29))
  (Variables|DinamicVariables|Rotation|SetTargetPitch Pitch)
  (bind _output_get (Variables|DinamicVariables|Rotation|SetCurrentPitch (Math|Interpolation|FInterpTo (Variables|DinamicVariables|Rotation|GetCurrentPitch) (Variables|DinamicVariables|Rotation|GetTargetPitch) DeltaSeconds 1e+01)))
  (Transformation|AddActorLocalRotation (Math|Rotator|MakeRotator 0.0 (* _output_get DeltaSeconds 15.0) 0.0) false false)
  (Transformation|SetRelativeRotation (Variables|Default|GetSM_elevatorR) (Math|Rotator|MakeRotator 0.0 (Math|Float|MapRangeClamped (Variables|DinamicVariables|Rotation|GetCurrentPitch) -1.0 1.0 (Variables|Constansts|Controller|GetMaxElevtorPitch) (Utilities|NegateFloat (Variables|Constansts|Controller|GetMaxElevtorPitch))) 0.0) false false)
  (Transformation|SetRelativeRotation (Variables|Default|GetSM_elevatorL) (Math|Rotator|MakeRotator 0.0 (Math|Float|MapRangeClamped (Variables|DinamicVariables|Rotation|GetCurrentPitch) -1.0 1.0 (Variables|Constansts|Controller|GetMaxElevtorPitch) (Utilities|NegateFloat (Variables|Constansts|Controller|GetMaxElevtorPitch))) 0.0) false false))

(fn UpdateRoll
  (params (DeltaSeconds :type Float%20%28single-precision%29) (Roll :type Float%20%28single-precision%29))
  (Variables|DinamicVariables|Rotation|SetTargetRoll Roll)
  (bind _output_get (Variables|DinamicVariables|Rotation|SetCurrentRoll (Math|Interpolation|FInterpTo (Variables|DinamicVariables|Rotation|GetCurrentRoll) (Variables|DinamicVariables|Rotation|GetTargetRoll) DeltaSeconds 1e+01)))
  (Transformation|AddActorLocalRotation (Math|Rotator|MakeRotator (* _output_get DeltaSeconds 15.0) 0.0 0.0) false false)
  (Transformation|SetRelativeRotation (Variables|Default|GetSM_aileronL) (Math|Rotator|MakeRotator 0.0 (Math|Float|MapRangeClamped (Variables|DinamicVariables|Rotation|GetCurrentRoll) -1.0 1.0 (Utilities|NegateFloat (Variables|Constansts|Controller|GetMaxAileronPitch)) (Variables|Constansts|Controller|GetMaxAileronPitch)) 0.0) false false)
  (Transformation|SetRelativeRotation (Variables|Default|GetSM_aileronR) (Math|Rotator|MakeRotator 0.0 (Math|Float|MapRangeClamped (Variables|DinamicVariables|Rotation|GetCurrentRoll) -1.0 1.0 (Variables|Constansts|Controller|GetMaxAileronPitch) (Utilities|NegateFloat (Variables|Constansts|Controller|GetMaxAileronPitch))) 0.0) false false))

(fn PrintVariebles
  (Utilities|FlowControl|Sequence
    (:then_0
      (Development|PrintString (Utilities|String|Append "TrustSpeed:" (Utilities|String|ToString(Float) (Variables|DinamicVariables|GetTrustSpeed))) true true "(R=0.000000,G=0.660000,B=1.000000,A=1.000000)" 0.0))
    (:then_1
      (Development|PrintString (Utilities|String|Append "CurrentSpeed:" (Utilities|String|ToString(Float) (Variables|DinamicVariables|GetCurrentSpeed))) true true "(R=0.000000,G=0.660000,B=1.000000,A=1.000000)" 0.0))
    (:then_2
      (Development|PrintString (Utilities|String|Append "ApplyedGravity:" (Utilities|String|ToString(Float) (Variables|DinamicVariables|GetApplyedGravity))) true true "(R=0.000000,G=0.660000,B=1.000000,A=1.000000)" 0.0))))

(fn UpdateTruster)