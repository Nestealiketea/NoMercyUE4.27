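; Server game mode that runs a timed match for the player controllers it collects on login.
; Countdown fires once, showing each player a countdown, then after a delay unfreezes them and shows in-game timers.
; A looping one-second timer decrements the time stored in the game state, pausing and freezing all players at zero.
; A separate SpawnPlayers function creates local players and possesses spawned characters.
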(event Custom|Countdown
  (if (not (Variables|Default|GetStarted))
    (for _array_element (Variables|Default|GetPlayers)
      (Default|ShowCountDown _array_element))
    (Variables|Default|SetStarted true)
    (Utilities|FlowControl|Delay 6.0)
    (CallFunction|Unfreeze)))

(event Custom|ShowTimers
  (for _array_element (Variables|Default|GetPlayers)
    (Default|ShowTimerinGame _array_element)))

(event Custom|Freeze
  (for _array_element (Variables|Default|GetPlayers)
    (Default|Freeze _array_element)))

(event Custom|Count
  (bind _result (Math|Integer|DecrementInt (Variables|/Game/Server/Blueprints/myGS_Server.myGS_Server_C|GetcurrentTime (Variables|Default|GetMy%20GS%20Server)))
    (:%20%20
      (if (== _result 0)
        (Utilities|Time|PauseTimerbyHandle (stale Custom|UnFreeze _returnvalue))
        (CallFunction|Freeze)))))

(event Custom|UnFreeze
  (for _array_element (Variables|Default|GetPlayers)
    (Default|Unfreeze _array_element))
  (Variables|/Game/Server/Blueprints/myGS_Server.myGS_Server_C|SetcurrentTime (Variables|Default|GetMy%20GS%20Server) (Variables|Default|GetmatchTime))
  (bind _returnvalue (Utilities|Time|SetTimerbyEvent (delegate Custom|Count) 1.0 true))
  (CallFunction|ShowTimers))

(event EventBeginPlay
  (bind _asmy_gs_server (Utilities|Casting|CastTomyGS_Server (Game|GetGameState)))
  (Variables|Default|SetMy%20GS%20Server _asmy_gs_server))

(event EventTick
  (params (DeltaSeconds :type Float%20%28single-precision%29)))

(event EventPostLogin
  (params (NewPlayer :type Player%20Controller%20Object%20Reference))
  (bind _ascontroller_bp (Utilities|Casting|CastToController_BP NewPlayer))
  (Utilities|Array|Add (Variables|Default|GetPlayers) _ascontroller_bp))

(fn ConstructionScript)

(fn SpawnPlayers
  (for _index (range 1 2)
    (Class|GameplayStatics|CreatePlayer _index))
  (for _index_2 (range 0 2)
    (bind _returnvalue (Game|SpawnActorfromClass "/Game/Player/Blueprints/Character/Blueprints/Character_BP.Character_BP_C" (Math|Transform|MakeTransform "0.000000, 0,0.000000") "Undefined" 0 _index_2 0))
    (Pawn|Possess (Game|GetPlayerController _index_2) _returnvalue)))