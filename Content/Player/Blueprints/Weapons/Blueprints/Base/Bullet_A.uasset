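; Bullet_A is a weapon projectile actor that deals fixed damage to whatever it hits.
; On BeginPlay a timeline drives the Bullet component's scale, and its update chain also leads into a delayed self-destroy that limits lifetime.
; On Hit it destroys itself, spawns an Impuct actor at the hit location and applies damage, passing the hit actor as its own damage causer.
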(event EventBeginPlay
  (bind _bullet (Variables|Default|GetBullet))
  (bind _newtrack_1 (Timeline|Timeline_0 Play)
    (:Update
      (Transformation|SetWorldTransform _bullet (Math|Transform|MakeTransform (Transformation|GetWorldLocation _bullet) (Transformation|GetWorldRotation _bullet) _newtrack_1) false false)
      (Utilities|FlowControl|Delay 1e+01)
      (Actor|DestroyActor))))

(event Collision|EventActorBeginOverlap
  (params (OtherActor :type Actor%20Object%20Reference)))

(event EventTick
  (params (DeltaSeconds :type Float%20%28single-precision%29)))

(event Collision|EventHit
  (params (MyComp :type Primitive%20Component%20Object%20Reference) (Other :type Actor%20Object%20Reference) (OtherComp :type Primitive%20Component%20Object%20Reference) (bSelfMoved :type Boolean) (HitLocation :type Vector :default "0, 0, 0") (HitNormal :type Vector :default "0, 0, 0") (NormalImpulse :type Vector :default "0, 0, 0") (Hit :type Hit%20Result%20Structure%20%28by%20ref%29))
  (bind _hitactor (Collision|BreakHitResult Hit))
  (Actor|DestroyActor)
  (Game|SpawnActorfromClass "/Game/Player/Blueprints/Weapons/Blueprints/Base/Impuct.Impuct_C" (Math|Conversions|ToTransform(Vector) HitLocation) "AlwaysSpawn" 0 0) ; Spawn projectile
  (Game|Damage|ApplyDamage _hitactor 6e+01 0 _hitactor "/Script/Engine.DamageType"))

(fn ConstructionScript)