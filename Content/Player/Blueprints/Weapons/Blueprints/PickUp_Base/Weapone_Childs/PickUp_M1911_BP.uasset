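; M1911 weapon pickup, a child Blueprint that adds suppressor handling and pistol firing animation.
; BeginPlay spawns a Suppressor_BP, and Tick re-attaches it to skeletal mesh socket "SU" or "0" depending on IsSU.
; GunAnimShoot animates firing procedurally by stepping the hammer and slide (Zatvor) variables in M1911_ABP with short delays.
; ServerRemovePickUp destroys the pickup actor.
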(event EventBeginPlay
  (bind _returnvalue (Game|SpawnActorfromClass "/Game/Player/Blueprints/Weapons/Blueprints/Ammunition/Suppressor_BP.Suppressor_BP_C" (Math|Transform|MakeTransform "0, 0, 0") "Undefined" 0 0))
  (Transformation|AttachComponentToComponent _returnvalue (Variables|Default|GetSkeletalMesh) "0" "KeepRelative" "KeepRelative" "KeepRelative" true))

(event EventGunAnimShoot
  (bind _skeletalmesh (Variables|Default|GetSkeletalMesh))
  (bind _returnvalue (Components|SkeletalMesh|GetAnimInstance _skeletalmesh))
  (bind _asm1911_abp (Utilities|Casting|CastToM1911_ABP _returnvalue))
  (Variables|/Game/Player/Blueprints/Weapons/Anim-Blueprints/M1911_ABP.M1911_ABP_C|SetHammer_0 _asm1911_abp 0.0)
  (Utilities|FlowControl|Delay 0.05)
  (Variables|/Game/Player/Blueprints/Weapons/Anim-Blueprints/M1911_ABP.M1911_ABP_C|SetHammer_0 _asm1911_abp -65.0)
  (Variables|/Game/Player/Blueprints/Weapons/Anim-Blueprints/M1911_ABP.M1911_ABP_C|Setzatvor_0 _asm1911_abp -5.5)
  (Utilities|FlowControl|Delay 0.05)
  (Variables|/Game/Player/Blueprints/Weapons/Anim-Blueprints/M1911_ABP.M1911_ABP_C|Setzatvor_0 _asm1911_abp 0.0))

(event EventTick
  (params (DeltaSeconds :type Float%20%28single-precision%29))
  (bind _skeletalmesh (Variables|Default|GetSkeletalMesh))
  (if (Variables|Default|GetIsSU?)
    (Transformation|AttachComponentToComponent (stale EventBeginPlay _returnvalue) _skeletalmesh "SU" "KeepRelative" "KeepRelative" "KeepRelative" true)
    (else
      (Transformation|AttachComponentToComponent (stale EventBeginPlay _returnvalue) _skeletalmesh "0" "KeepRelative" "KeepRelative" "KeepRelative" true))))

(event EventServerRemovePickUp
  (Actor|DestroyActor))

(fn ConstructionScript
  (|CallParentFunction))