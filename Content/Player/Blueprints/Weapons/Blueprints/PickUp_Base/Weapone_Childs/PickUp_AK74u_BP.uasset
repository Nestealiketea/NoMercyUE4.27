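; AK74u weapon child of the pickup base, covering the gun's visuals, removal and damage.
; Tick sets or clears the suppressor static mesh from the IsSU flag, while unconnected nodes for spawning and attaching a suppressor actor never run.
; GunAnimShoot briefly kicks the bolt back through the Zatvor0 variable on the AK74u anim blueprint.
; ServerRemovePickUp destroys the actor, and Damage applies point damage with the instigator's controller.
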(event EventBeginPlay)

(event EventGunAnimShoot
  (bind _skeletalmesh (Variables|Default|GetSkeletalMesh))
  (bind _returnvalue (Components|SkeletalMesh|GetAnimInstance _skeletalmesh))
  (bind _asak74u_abp (Utilities|Casting|CastToAK74u_ABP _returnvalue))
  (Variables|/Game/Player/Blueprints/Weapons/Anim-Blueprints/AK74u_ABP.AK74u_ABP_C|Setzatvor_0 _asak74u_abp -14.0)
  (Utilities|FlowControl|Delay 0.05)
  (Variables|/Game/Player/Blueprints/Weapons/Anim-Blueprints/AK74u_ABP.AK74u_ABP_C|Setzatvor_0 _asak74u_abp 0.0))

(event EventTick
  (params (DeltaSeconds :type Float%20%28single-precision%29))
  (bind _suppressor (Variables|Default|GetSuppressor))
  (if (Variables|Default|GetIsSU?)
    (Components|StaticMesh|SetStaticMesh _suppressor "/Game/Player/Blueprints/Weapons/Meshes/Accessories/SM_Suppressor5.SM_Suppressor5")
    (else
      (Components|StaticMesh|SetStaticMesh _suppressor 0))))

(event EventServerRemovePickUp
  (Actor|DestroyActor))

(fn ConstructionScript
  (|CallParentFunction))