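; PickUp_BP is a base pickup for player weapons, with mostly empty hooks for child weapons to fill in.
; Input-style events for firing, weapon mode and suppressor forward to Server events, and simple functions return its self reference, blend space and weapon type.
; On authority, a Sphere overlap with a Player-tagged actor passes the pickup to SetPickUpMessage after a short delay.
; ServerCollisionDisable, despite its name, sets the sphere to QueryAndPhysics.
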(event OnComponentBeginOverlap(Sphere)
  (params (OverlappedComponent :type Primitive%20Component%20Object%20Reference) (OtherActor :type Actor%20Object%20Reference) (OtherComp :type Primitive%20Component%20Object%20Reference) (OtherBodyIndex :type Integer) (bFromSweep :type Boolean) (SweepResult :type Hit%20Result%20Structure%20%28by%20ref%29))
  (Networking|SwitchHasAuthority
    (:Authority
      (if (Actor|ActorHasTag OtherActor "Player")
        (Utilities|FlowControl|Delay 0.1)
        (Class|CharcterBPI|SetPickUp(Message) OtherActor self)))))

(event OnComponentEndOverlap(Sphere)
  (params (OverlappedComponent :type Primitive%20Component%20Object%20Reference) (OtherActor :type Actor%20Object%20Reference) (OtherComp :type Primitive%20Component%20Object%20Reference) (OtherBodyIndex :type Integer)))

(event Custom|Server%20Suppressor)

(event Custom|Server%20Remove%20PickUp)

(event Custom|Server%20Stop%20Shoot)

(event Custom|Server%20Shoot)

(event Custom|Server%20Start%20Shoot)

(event Custom|Server%20Collision%20Disable
  (Collision|SetCollisionEnabled (Variables|Components|GetSphere) "QueryAndPhysics"))

(event Custom|Server%20Weapone%20Mode)

(event EventWeaponeMode
  (CallFunction|ServerWeaponeMode))

(event EventTick
  (params (DeltaSeconds :type Float%20%28single-precision%29)))

(event EventWeaponeSU
  (CallFunction|ServerSuppressor))

(event EventStartFire
  (CallFunction|ServerStartShoot))

(event EventStopFire
  (CallFunction|ServerStopShoot))

(event EventShoot
  (CallFunction|ServerShoot))

(event EventBeginPlay)

(fn ConstructionScript)

(fn BlendSpaceInt
  (return (Variables|Default|GetBlandSpace)))

(fn PickUpRef
  (return self))

(fn WeaponeType
  (return "NewEnumerator0"))