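; PM is a player weapon Blueprint that hides its empty-magazine bone on BeginPlay and handles its own physics state and removal.
; A single event with a collision setting and boolean flags sets mesh collision, optionally enables physics simulation, and destroys the actor.
; When simulation and timed destruction are both requested, a 30-second delay precedes the destroy.
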(event Custom|Symulate%20PH/Destroy/Collision
  (params (Collision :type ECollisionEnabled%20Enum :default "NoCollision") (bSimulate :type Boolean) (Destroy :type Boolean) (Destroy%20after%2030s :type Boolean))
  (bind _pm (Variables|Default|GetPM))
  (Collision|SetCollisionEnabled _pm Collision)
  (if bSimulate
    (Physics|SetSimulatePhysics _pm bSimulate)
    (if Destroy%20after%2030s
      (Utilities|FlowControl|Delay 3e+01)))
  (if (or Destroy Destroy%20after%2030s)
    (Actor|DestroyActor)))

(event EventBeginPlay
  (Components|SkinnedMesh|HideBonebyName (Variables|Default|GetPM) "b_gun_mag_empty" "PBO_None"))

(event Collision|EventActorBeginOverlap
  (params (OtherActor :type Actor%20Object%20Reference)))

(event EventTick
  (params (DeltaSeconds :type Float%20%28single-precision%29)))

(fn ConstructionScript)