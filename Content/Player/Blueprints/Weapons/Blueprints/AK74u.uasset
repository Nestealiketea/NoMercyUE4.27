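; AK74u weapon actor Blueprint handling the rifle's firing effects and its physics and cleanup state.
; ServerShoot briefly offsets the bolt (Zatvor0) through the AK74u_ABP anim instance, then spawns attached muzzle flash and shell eject emitters and plays the fire sound.
; A utility event sets mesh collision, optionally enables physics simulation, and destroys the actor immediately or after a delay.
; No hit or damage logic is present.
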(event Custom|Server%20Shoot
  (bind _ak74u (Variables|Default|GetAK74U))
  (bind _returnvalue (Components|SkeletalMesh|GetAnimInstance _ak74u))
  (bind _asak74u_abp (Utilities|Casting|CastToAK74u_ABP _returnvalue))
  (Variables|/Game/Player/Blueprints/Weapons/Anim-Blueprints/AK74u_ABP.AK74u_ABP_C|Setzatvor_0 _asak74u_abp -14.0)
  (Utilities|FlowControl|Delay 0.05)
  (Variables|/Game/Player/Blueprints/Weapons/Anim-Blueprints/AK74u_ABP.AK74u_ABP_C|Setzatvor_0 _asak74u_abp 0.0)
  (Effects|SpawnEmitterAttached "/Game/Player/Particles/Emitters/P_AK74u_Muzzleflash.P_AK74u_Muzzleflash" (Variables|Default|GetMuzzle) "None")
  (Effects|SpawnEmitterAttached "/Game/Player/Particles/Emitters/P_AK74u_ShellEject.P_AK74u_ShellEject" (Variables|Default|GetSleeve) "None")
  (Audio|PlaySoundatLocation "/Game/Player/Audio/Rifle/RifleB_Fire_Cue.RifleB_Fire_Cue" (Transformation|GetWorldLocation (Variables|Default|GetMuzzle)) "0, 0, 0" 1.0 1.0 0.0 0 0 0))

(event Custom|Symulate%20PH/Destroy/Collision
  (params (Collision :type ECollisionEnabled%20Enum :default "NoCollision") (bSimulate :type Boolean) (Destroy :type Boolean) (Destroy%20after%2030s :type Boolean))
  (bind _ak74u (Variables|Default|GetAK74U))
  (Collision|SetCollisionEnabled _ak74u Collision)
  (if bSimulate
    (Physics|SetSimulatePhysics _ak74u bSimulate)
    (if Destroy%20after%2030s
      (Utilities|FlowControl|Delay 3e+01)))
  (if (or Destroy Destroy%20after%2030s)
    (Actor|DestroyActor)))

(event EventBeginPlay)

(fn ConstructionScript)