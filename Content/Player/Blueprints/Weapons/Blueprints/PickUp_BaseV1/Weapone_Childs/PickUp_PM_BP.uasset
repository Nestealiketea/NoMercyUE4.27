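; PM pistol weapon pickup, apparently a child of the PickUp_BaseV1 weapon base, that adds pistol-specific mesh setup and animation.
; On BeginPlay it hides the empty-magazine bone on the skeletal mesh.
; The Anim event fakes a firing cycle by setting hammer and slide (Zatvor) variables on PM_ABP with short delays, rather than playing a montage.
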(event EventBeginPlay
  (Components|SkinnedMesh|HideBonebyName (Variables|Default|GetSkeletalMesh) "b_gun_mag_empty" "PBO_None"))

(event Collision|EventActorBeginOverlap
  (params (OtherActor :type Actor%20Object%20Reference)))

(event EventTick
  (params (DeltaSeconds :type Float%20%28single-precision%29)))

(event EventAnim
  (bind _skeletalmesh (Variables|Default|GetSkeletalMesh))
  (bind _returnvalue (Components|SkeletalMesh|GetAnimInstance _skeletalmesh))
  (bind _aspm_abp (Utilities|Casting|CastToPM_ABP _returnvalue))
  (Variables|/Game/Player/Blueprints/Weapons/Anim-Blueprints/PM_ABP.PM_ABP_C|SetHammer_0 _aspm_abp 0.0)
  (Utilities|FlowControl|Delay 0.08)
  (Variables|/Game/Player/Blueprints/Weapons/Anim-Blueprints/PM_ABP.PM_ABP_C|SetHammer_0 _aspm_abp -55.0)
  (Variables|/Game/Player/Blueprints/Weapons/Anim-Blueprints/PM_ABP.PM_ABP_C|Setzatvor_0 _aspm_abp -3.8)
  (Utilities|FlowControl|Delay 0.05)
  (Variables|/Game/Player/Blueprints/Weapons/Anim-Blueprints/PM_ABP.PM_ABP_C|Setzatvor_0 _aspm_abp 0.0))

(fn ConstructionScript
  (|CallParentFunction))