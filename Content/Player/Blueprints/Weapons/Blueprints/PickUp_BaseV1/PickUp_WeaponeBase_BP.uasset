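; Base weapon pickup Blueprint that handles hitscan shooting, with toggles for fire mode and suppressor.
; Server-named start and stop events fire a shot, then run or clear a looping timer for automatic fire.
; Each shot plays suppressor-aware muzzle effects and sound, shell ejection and camera shake, then line-traces from the camera.
; The hit's physical surface selects body-part damage, applied as point damage using camera location as hit direction.
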(event Custom|Multi%20Emitter/Sound
  (params (SU :type Boolean) (Muzzle%20Emitter :type Particle%20System%20Object%20Reference) (Muzzle%20Emitter%20SU :type Particle%20System%20Object%20Reference) (AttachToComponent :type Scene%20Component%20Object%20Reference) (Muzzle%20PointName :type Name) (Muzzle%20PointName%20SU :type Name) (Muzzle%20Scale :type Vector) (Sleeve%20Emitter :type Particle%20System%20Object%20Reference) (Sleeve%20PointName :type Name) (Sleeve%20Scale :type Vector) (Sound :type Sound%20Base%20Object%20Reference) (Sound%20SU :type Sound%20Base%20Object%20Reference))
  (Effects|SpawnEmitterAttached (select SU Muzzle%20Emitter%20SU Muzzle%20Emitter) AttachToComponent (select SU Muzzle%20PointName%20SU Muzzle%20PointName) "0, 0, 0" "0, 0, 0" Muzzle%20Scale)
  (Effects|SpawnEmitterAttached Sleeve%20Emitter AttachToComponent Sleeve%20PointName "0, 0, 0" "0, 0, 0" Sleeve%20Scale)
  (Audio|PlaySoundatLocation (select SU Sound%20SU Sound) (Transformation|GetActorLocation) "0, 0, 0" 1.0 1.0 0.0 0 0 0))

(event Custom|Gun_Anim_Shoot)

(event EventServerShoot
  (bind _camera (Variables|Components|GetCamera))
  (CallFunction|GunAnimShoot)
  (CallFunction|MultiEmitter/Sound (Variables|Default|GetIsSU?) (Variables|Default|GetMuzzle%20Emitter) (Variables|Default|GetMuzzle%20Emitter%20SU) (Variables|Default|GetSkeletalMesh) (Variables|Default|GetMuzzle%20Point%20Name) (Variables|Default|GetMuzzle%20Point%20Name%20SU) (Variables|Default|GetMuzzle%20Scale) (Variables|Default|GetSleeve%20Emitter) (Variables|Default|GetSleeve%20Point%20Name) (Variables|Default|GetSleeve%20Scale) (Variables|Default|GetSound) (Variables|Default|GetSound%20SU))
  (Class|ControllerBPI|CameraShake(Message) (Game|GetInstigatorController) (Variables|Default|GetShoot%20CS) (Variables|Default|GetMontage) (Variables|Default|GetPlay%20Rate) (Variables|Default|GetMin%20Pitch) (Variables|Default|GetMax%20Pitch) (Variables|Default|GetMin%20Yaw) (Variables|Default|GetMax%20Yaw))
  (Variables|Default|SetCamera%20Location (Transformation|GetWorldLocation _camera))
  (Variables|Default|SetCamera%20Rotation (Transformation|GetWorldRotation _camera))
  (bind (_outhit _returnvalue) (Collision|LineTraceByChannel (Variables|Default|GetCamera%20Location) (+ (Variables|Default|GetCamera%20Location) (* (Math|Vector|GetForwardVector (Variables|Default|GetCamera%20Rotation)) (Variables|Default|GetBullet%20Distance))) "TraceTypeQuery1" true (Utilities|Array|MakeArray (Components|GetOwner) self) "None" true "(R=1.000000,G=0.000000,B=0.000000,A=1.000000)" "(R=0.000000,G=1.000000,B=0.000000,A=1.000000)" 1.0))
  (if _returnvalue
    (switch Utilities|FlowControl|Switch|SwitchonEPhysicalSurface (Variables|/Script/PhysicsCore.PhysicalMaterial|GetSurfaceType (.PhysMat (Collision|BreakHitResult _outhit)))
      (:SurfaceType_Default
        (Utilities|Damage (.HitActor (Collision|BreakHitResult _outhit)) _outhit (Variables|Damage|GetBase%20Damage) (.ImpactNormal (Collision|BreakHitResult _outhit))))
      (:SurfaceType1
        (Utilities|Damage (.HitActor (Collision|BreakHitResult _outhit)) _outhit (Variables|Damage|GetHead%20Damage) (.ImpactNormal (Collision|BreakHitResult _outhit))))
      (:SurfaceType2
        (Utilities|Damage (.HitActor (Collision|BreakHitResult _outhit)) _outhit (Variables|Damage|GetBody%20Damage) (.ImpactNormal (Collision|BreakHitResult _outhit))))
      (:SurfaceType3
        (Utilities|Damage (.HitActor (Collision|BreakHitResult _outhit)) _outhit (Variables|Damage|GetPart1%20Damage) (.ImpactNormal (Collision|BreakHitResult _outhit))))
      (:SurfaceType4
        (Utilities|Damage (.HitActor (Collision|BreakHitResult _outhit)) _outhit (Variables|Damage|GetPart2%20Damage) (.ImpactNormal (Collision|BreakHitResult _outhit)))))))

(event EventPlayerCameraRef
  (params (Camera :type Camera%20Component%20Object%20Reference))
  (Variables|Components|SetCamera Camera))

(event EventServerWeaponeMode
  (if (stale _output_get)
    (Variables|Default|SetIsAutomatic? false)
    (else
      (bind _output_get (Variables|Default|SetIsAutomatic? true)))))

(event EventServerStartShoot
  (CallFunction|ServerShoot)
  (if (Variables|Default|GetCan%20Be%20Auto?)
    (if (Variables|Default|GetIsAutomatic?)
      (bind _returnvalue (Utilities|Time|SetTimerbyEvent (delegate EventServerShoot) (Variables|Default|GetTBS) true))
      (Variables|Default|SetFiring%20Timer _returnvalue))))

(event EventServerStopShoot
  (Utilities|Time|ClearandInvalidateTimerbyHandle (Variables|Default|GetFiring%20Timer)))

(event EventServerSuppressor
  (if (stale _output_get)
    (Variables|Default|SetIsSU? false)
    (else
      (bind _output_get (Variables|Default|SetIsSU? true)))))

(fn ConstructionScript
  (|CallParentFunction))

(fn OnRepCameraLocation)