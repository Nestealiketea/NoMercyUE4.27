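; Slot-one weapon actor, apparently an AK-74u, with fire mode and suppressor toggles, physics switching and destruction.
; StartShooting spawns a bullet at the muzzle, kicks the bolt through AnimBP variables, spawns muzzle and casing effects, and messages camera shake to the instigator's controller.
; The suppressor flag selects muzzle effect and sound, and Tick reapplies its mesh.
; The looping automatic-fire timer is disconnected, and the shot passes no sounds.
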(event Custom|Multi%20Emitter/Sound
  (params (SU :type Boolean) (Muzzle%20Emitter :type Particle%20System%20Object%20Reference) (Muzzle%20Emitter%20SU :type Particle%20System%20Object%20Reference) (AttachToComponent :type Scene%20Component%20Object%20Reference) (Muzzle%20PointName :type Name) (Muzzle%20PointName%20SU :type Name) (Muzzle%20Scale :type Vector) (Sleeve%20Emitter :type Particle%20System%20Object%20Reference) (Sleeve%20PointName :type Name) (Sleeve%20Scale :type Vector) (Sound :type Sound%20Base%20Object%20Reference) (Sound%20SU :type Sound%20Base%20Object%20Reference))
  (Effects|SpawnEmitterAttached (select SU Muzzle%20Emitter%20SU Muzzle%20Emitter) AttachToComponent (select SU Muzzle%20PointName%20SU Muzzle%20PointName) "0, 0, 0" "0, 0, 0" Muzzle%20Scale)
  (Effects|SpawnEmitterAttached Sleeve%20Emitter AttachToComponent Sleeve%20PointName "0, 0, 0" "0, 0, 0" Sleeve%20Scale)
  (Audio|PlaySoundatLocation (select SU Sound%20SU Sound) (Transformation|GetActorLocation) "0, 0, 0" 1.0 1.0 0.0 0 0 0))

(event Custom|Start%20Shooting
  (bind _asak74u_abp (Utilities|AnimBp))
  (bind _arrow (Variables|Default|GetArrow))
  (Game|SpawnActorfromClass "/Game/Player/Blueprints/Weapons/Blueprints/Bullet_A.Bullet_A_C" (Math|Transform|MakeTransform (Transformation|GetSocketLocation _arrow "Muzzle") (Transformation|GetSocketRotation _arrow "Muzzle")) "AlwaysSpawn" 0 0)
  (Variables|/Game/Player/Blueprints/Weapons/Anim-Blueprints/AK74u_ABP.AK74u_ABP_C|Setzatvor_0 _asak74u_abp -14.0)
  (Utilities|FlowControl|Delay (/ (Variables|Default|GetShoot%20Time) 2.0))
  (Variables|/Game/Player/Blueprints/Weapons/Anim-Blueprints/AK74u_ABP.AK74u_ABP_C|Setzatvor_0 _asak74u_abp 0.0)
  (CallFunction|MultiEmitter/Sound (Variables|Default|GetIsSU?) (Variables|Default|GetMuzzle%20Emitter) (Variables|Default|GetMuzzle%20Emitter%20SU) (Variables|Default|GetSkeletalMesh) (Variables|Default|GetMuzzle%20Point%20Name) (Variables|Default|GetMuzzle%20Point%20Name%20SU) (Variables|Default|GetMuzzle%20Scale) (Variables|Default|GetSleeve%20Emitter) (Variables|Default|GetSleeve%20Point%20Name) (Variables|Default|GetSleeve%20Scale))
  (Class|ControllerBPI|CameraShake(Message) (Game|GetInstigatorController) (Variables|Default|GetShoot%20CS) (Variables|Default|GetMontage) (Variables|Default|GetPlay%20Rate) (Variables|Default|GetMin%20Pitch) (Variables|Default|GetMax%20Pitch) (Variables|Default|GetMin%20Yaw) (Variables|Default|GetMax%20Yaw)))

(event Custom|Destroy_AK
  (Actor|DestroyActor))

(event Custom|End%20Shooting
  (Utilities|Time|ClearandInvalidateTimerbyHandle (Variables|Default|GetFiring%20Timer)))

(event Custom|Weapone%20Mode
  (bind _asak74u_abp (Utilities|AnimBp))
  (if (stale _output_get)
    (Variables|Default|SetIsAutomatic? false)
    (Variables|/Game/Player/Blueprints/Weapons/Anim-Blueprints/AK74u_ABP.AK74u_ABP_C|Setfiremode_0 _asak74u_abp 0.0)
    (else
      (bind _output_get (Variables|Default|SetIsAutomatic? true))
      (Variables|/Game/Player/Blueprints/Weapons/Anim-Blueprints/AK74u_ABP.AK74u_ABP_C|Setfiremode_0 _asak74u_abp -7.0))))

(event Custom|Simulate_PH_AK
  (params (Simulate :type Boolean) (Collision :type ECollisionEnabled%20Enum :default "NoCollision"))
  (bind _skeletalmesh (Variables|Default|GetSkeletalMesh))
  (Physics|SetSimulatePhysics _skeletalmesh Simulate)
  (Collision|SetCollisionEnabled _skeletalmesh Collision))

(event Custom|Suppressor%20Mode
  (if (stale _output_get)
    (Variables|Default|SetIsSU? false)
    (else
      (bind _output_get (Variables|Default|SetIsSU? true)))))

(event EventTick
  (params (DeltaSeconds :type Float%20%28single-precision%29))
  (bind _suppressor (Variables|Default|GetSuppressor))
  (if (Variables|Default|GetIsSU?)
    (Components|StaticMesh|SetStaticMesh _suppressor "/Game/Player/Blueprints/Weapons/Meshes/Accessories/SM_Suppressor5.SM_Suppressor5")
    (else
      (Components|StaticMesh|SetStaticMesh _suppressor 0))))

(event EventBeginPlay)

(fn ConstructionScript)