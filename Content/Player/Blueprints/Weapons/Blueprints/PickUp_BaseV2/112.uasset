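; Weapon Blueprint that fires automatically from BeginPlay.
; A looping timer calls StartShooting at a fixed interval, spawning a Bullet_A at the skeletal mesh's Muzzle socket with that socket's rotation, regardless of collision.
; EndShooting clears the stored timer handle to stop the fire loop.
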(event Custom|Start%20Shooting
  (bind _skeletalmesh (Variables|Default|GetSkeletalMesh))
  (Game|SpawnActorfromClass "/Game/Player/Blueprints/Weapons/Blueprints/Bullet_A.Bullet_A_C" (Math|Transform|MakeTransform (Transformation|GetSocketLocation _skeletalmesh "Muzzle") (Transformation|GetSocketRotation _skeletalmesh "Muzzle")) "AlwaysSpawn" 0 0))

(event Custom|End%20Shooting
  (Utilities|Time|ClearandInvalidateTimerbyHandle (Variables|Default|GetFiring%20Timer)))

(event EventTick
  (params (DeltaSeconds :type Float%20%28single-precision%29)))

(event EventBeginPlay
  (bind _returnvalue (Utilities|Time|SetTimerbyEvent (delegate Custom|Start%20Shooting) 0.3 true))
  (Variables|Default|SetFiring%20Timer _returnvalue))

(fn ConstructionScript)