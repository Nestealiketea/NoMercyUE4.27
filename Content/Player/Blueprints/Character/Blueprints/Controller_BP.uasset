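; Player controller that manages a multiplayer player's HUD, scoreboard, exit menu, match timer widgets and client camera shakes.
; Tab shows a scoreboard that a fast looping timer rebuilds from every Character_BP and its player state's name, kills and deaths, plus health.
; Escape or End opens the cursor-driven exit menu, and Enter starts the server game mode's countdown.
; Freeze and UnFreeze both enable pawn input, and several functions are empty stubs.
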(event Custom|23
  (params (Target :type Player%20Controller%20Object%20Reference) (Shake :type Camera%20Shake%20Base%20Class%20Reference) (Scale :type Float%20%28single-precision%29)))

(event Custom|Client%20Players_Info%20T
  ;[1 1 1] UI
  (bind _returnvalue (UserInterface|CreateWidget "/Game/Player/Blueprints/Character/HUD/Players_Informatio_HUD.Players_Informatio_HUD_C"))
  (UserInterface|Viewport|AddtoViewport _returnvalue 0))

(event Custom|Client%20Players_Info%20F
  ;[1 1 1] UI
  (Widget|RemovefromParent (stale Custom|Client%20Players_Info%20T _returnvalue)))

(event Custom|Inf%20Board%20Timer
  ;[1 1 1] UI
  (CallFunction|UpdateBoard (stale Custom|Client%20Players_Info%20T _returnvalue)))

(event Custom|Update_Board
  (params (InputObject :type Object%20Object%20Reference))
  (bind _asplayers_informatio_hud (Utilities|Casting|CastToPlayers_Informatio_HUD InputObject))
  (bind _playersinfo (Variables|/Game/Player/Blueprints/Character/HUD/Players_Informatio_HUD.Players_Informatio_HUD_C|GetPlayersInfo _asplayers_informatio_hud))
  ;[1 1 1] UI
  (Utilities|IsValid InputObject
    (:Is%20Valid
      (Widget|Panel|ClearChildren _playersinfo)
      (bind _outactors (Actor|GetAllActorsOfClass "/Game/Player/Blueprints/Character/Blueprints/Character_BP.Character_BP_C"))
      (for _array_element _outactors
        (bind _returnvalue (UserInterface|CreateWidget "/Game/Server/Blueprints/Create_PlayersInfo_HUD.Create_PlayersInfo_HUD_C" 0 (Utilities|Text|ToText(String) (PlayerState|GetPlayerName (Variables|/Script/Engine.Pawn|GetPlayerState _array_element))) (Variables|/Game/Server/Blueprints/myPlayerState.myPlayerState_C|GetKills (.AsMy%20Player%20State (Utilities|Casting|CastTomyPlayerState (Variables|/Script/Engine.Pawn|GetPlayerState _array_element)))) (Variables|/Game/Server/Blueprints/myPlayerState.myPlayerState_C|GetDeath (.AsMy%20Player%20State (Utilities|Casting|CastTomyPlayerState (Variables|/Script/Engine.Pawn|GetPlayerState _array_element)))) (Math|Float|Truncate (Variables|/Game/Player/Blueprints/Character/Blueprints/Character_BP.Character_BP_C|GetHealth _array_element))))
        (Widget|Panel|AddChild _playersinfo _returnvalue)))))

(event Custom|Client%20Exit_HUD%20F
  (bind _returnvalue (Game|GetPlayerController 0))
  ;[1 1 1] UI
  (Widget|RemovefromParent (stale Custom|Client%20Exit_HUD%20T _output_get))
  (Input|SetInputModeGameOnly _returnvalue)
  (Variables|/Script/Engine.PlayerController|SetbShowMouseCursor _returnvalue false))

(event Custom|Client%20Camera%20Shake
  (params (Shake :type Camera%20Shake%20Base%20Class%20Reference))
  (Game|Feedback|ClientStartCameraShake Shake 1.0 "CameraLocal" "0, 0, 0"))

(event Custom|Show%20HUD
  (bind _returnvalue (UserInterface|CreateWidget "/Game/Player/Blueprints/Character/HUD/Player_HUD.Player_HUD_C"))
  (UserInterface|Viewport|AddtoViewport _returnvalue 0))

(event Custom|Freeze
  (Input|EnableInput (Pawn|GetControlledPawn) self))

(event Custom|Client%20Exit_HUD%20T
  (bind _returnvalue (Game|GetPlayerController 0))
  ;[1 1 1] UI
  (bind _returnvalue_2 (UserInterface|CreateWidget "/Game/Player/Blueprints/Character/HUD/Exit_HUD.Exit_HUD_C"))
  (bind _output_get (Variables|Default|SetExit%20HUD _returnvalue_2))
  (UserInterface|Viewport|AddtoViewport _output_get 0)
  (Input|SetInputModeUIOnly _returnvalue _output_get "DoNotLock")
  (Variables|/Script/Engine.PlayerController|SetbShowMouseCursor _returnvalue true))

(event Custom|ShowTimerInGame
  (bind _returnvalue (UserInterface|CreateWidget "/Game/Test_Content/W_TimerInGame.W_TimerInGame_C"))
  (UserInterface|Viewport|AddtoViewport _returnvalue 0))

(event Custom|ShowCountDown
  (bind _returnvalue (UserInterface|CreateWidget "/Game/Test_Content/W_TimerBeforeGame.W_TimerBeforeGame_C"))
  (UserInterface|Viewport|AddtoViewport _returnvalue 0))

(event Custom|UnFreeze
  (Input|EnableInput (Pawn|GetControlledPawn) self))

(event EventBeginPlay
  (Utilities|Time|SetTimerbyEvent (delegate Custom|Inf%20Board%20Timer) 0.01 true)
  (CallFunction|ShowHUD))

(event EventCameraShake
  (params (Shake :type Matinee%20Camera%20Shake%20Class%20Reference) (Montage :type Anim%20Montage%20Object%20Reference) (Play%20Rate :type Float%20%28single-precision%29) (Min%20Pitch :type Float%20%28single-precision%29) (Max%20Pitch :type Float%20%28single-precision%29) (Min%20Yaw :type Float%20%28single-precision%29) (Max%20Yaw :type Float%20%28single-precision%29))
  (CallFunction|ClientCameraShake Shake))

(event Input|KeyboardEvents|Escape
  (params (Key :type Key%20Structure :default "None"))
  ;[1 1 1] UI
  (:Pressed
    (CallFunction|ClientExitHUDT)))

(event Input|KeyboardEvents|Enter
  (params (Key :type Key%20Structure :default "None"))
  (:Pressed
    (bind _asmy_gm_server (Utilities|Casting|CastTomyGM_Server (Game|GetGameMode)))
    (Default|Countdown _asmy_gm_server)))

(event Input|KeyboardEvents|End
  (params (Key :type Key%20Structure :default "None"))
  ;[1 1 1] UI
  (:Pressed
    (CallFunction|ClientExitHUDT)))

(event Input|KeyboardEvents|Tab
  (params (Key :type Key%20Structure :default "None"))
  ;[1 1 1] UI
  (:Pressed
    (CallFunction|ClientPlayersInfoT))
  (:Released
    (CallFunction|ClientPlayersInfoF)))

(fn ConstructionScript)

(fn FunctionHeadRotation)

(fn FunctionSpeedTransition)

(fn FunctionAxisSprint)

(fn OnRepValueY(Pitch))

(fn ServerSprint
  (params (Sprinting1 :type Boolean)))

(fn 12
  (params (Target1 :type Player%20Controller%20Object%20Reference) (Shake1 :type Camera%20Shake%20Base%20Class%20Reference) (Scale1 :type Float%20%28single-precision%29)))

(fn ControllerRef
  (return self))