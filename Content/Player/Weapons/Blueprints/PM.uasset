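; Makarov (PM) pistol weapon actor that handles the gun's firing cosmetics and its physics or removal.
; On begin play it hides the empty-magazine bone on the skeletal mesh.
; ServerShoot animates hammer and slide by setting PM_ABP variables between short delays, then spawns muzzle flash and shell eject emitters and plays the shot sound.
; A separate event sets collision, optionally enables physics, and destroys the actor, with an optional delay when simulating.
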(event Custom|Server%20Shoot
  (bind _pm (Variables|Default|GetPM))
  (bind _returnvalue (Components|SkeletalMesh|GetAnimInstance _pm))
  (bind _aspm_abp (Utilities|Casting|CastToPM_ABP _returnvalue))
  (Variables|/Game/Player/Weapons/Anim-Blueprints/PM_ABP.PM_ABP_C|SetHammer_0 _aspm_abp 0.0)
  (Utilities|FlowControl|Delay 0.05)
  (Variables|/Game/Player/Weapons/Anim-Blueprints/PM_ABP.PM_ABP_C|SetHammer_0 _aspm_abp -55.0)
  (Variables|/Game/Player/Weapons/Anim-Blueprints/PM_ABP.PM_ABP_C|Setzatvor_0 _aspm_abp -3.8)
  (Utilities|FlowControl|Delay 0.05)
  (Variables|/Game/Player/Weapons/Anim-Blueprints/PM_ABP.PM_ABP_C|Setzatvor_0 _aspm_abp 0.0)
  (Effects|SpawnEmitterAttached "/Game/Player/Particle/SleevesEmitters/Emitters/P_AK74u_Muzzleflash.P_AK74u_Muzzleflash" (Variables|Default|GetMuzzle) "None")
  (Effects|SpawnEmitterAttached "/Game/Player/Particle/SleevesEmitters/Emitters/P_PM_ShellEject.P_PM_ShellEject" (Variables|Default|GetSleeve) "None")
  (Audio|PlaySoundatLocation "/Game/Player/Audio/Sound/1911.1911" (Transformation|GetWorldLocation (Variables|Default|GetMuzzle)) "0, 0, 0" 1.0 1.0 0.1 0 0 0))

(event Custom|Symulate%20PH/Destroy/Collision
  (params (Collision :type ECollisionEnabled%20Enum :default "NoCollision") (bSimulate :type Boolean) (Destroy :type Boolean) (Destroy%20after%2030s :type Boolean))
  (bind _pm (Variables|Default|GetPM))
  (Collision|SetCollisionEnabled _pm Collision)
  (if bSimulate
    (Physics|SetSimulatePhysics _pm bSimulate)
    (if Destroy%20after%2030s
      (Utilities|FlowControl|Delay 3e+01)))
  (if (or Destroy Destroy%20after%2030s)
    (Actor|DestroyActor)))

(event EventBeginPlay
  (Components|SkinnedMesh|HideBonebyName (Variables|Default|GetPM) "b_gun_mag_empty" "PBO_None"))

(event Collision|EventActorBeginOverlap
  (params (OtherActor :type Actor%20Object%20Reference)))

(event EventTick
  (params (DeltaSeconds :type Float%20%28single-precision%29)))

(fn ConstructionScript)