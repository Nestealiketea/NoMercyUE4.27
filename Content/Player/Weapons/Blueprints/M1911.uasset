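; M1911 pistol weapon actor that handles the gun's firing visuals, sound and physics cleanup, with no hit or damage logic.
; ServerShoot steps the hammer and slide (Zatvor) variables in M1911_ABP through short delays, then spawns a borrowed AK74u muzzle flash, shell ejection and gunshot sound.
; A separate event sets mesh collision, optionally enables physics, and destroys the actor on request, with an optional delay when simulating.
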(event Custom|Server%20Shoot
  (bind _m1911 (Variables|Default|Getm1911))
  (bind _returnvalue (Components|SkeletalMesh|GetAnimInstance _m1911))
  (bind _asm1911_abp (Utilities|Casting|CastToM1911_ABP _returnvalue))
  (Variables|/Game/Player/Weapons/Anim-Blueprints/M1911_ABP.M1911_ABP_C|SetHammer_0 _asm1911_abp 0.0)
  (Utilities|FlowControl|Delay 0.05)
  (Variables|/Game/Player/Weapons/Anim-Blueprints/M1911_ABP.M1911_ABP_C|SetHammer_0 _asm1911_abp -65.0)
  (Variables|/Game/Player/Weapons/Anim-Blueprints/M1911_ABP.M1911_ABP_C|Setzatvor_0 _asm1911_abp -5.5)
  (Utilities|FlowControl|Delay 0.05)
  (Variables|/Game/Player/Weapons/Anim-Blueprints/M1911_ABP.M1911_ABP_C|Setzatvor_0 _asm1911_abp 0.0)
  (Effects|SpawnEmitterAttached "/Game/Player/Particle/SleevesEmitters/Emitters/P_AK74u_Muzzleflash.P_AK74u_Muzzleflash" (Variables|Default|GetMuzzle) "None")
  (Effects|SpawnEmitterAttached "/Game/Player/Particle/SleevesEmitters/Emitters/P_1911_ShellEject.P_1911_ShellEject" (Variables|Default|GetSleeve) "None")
  (Audio|PlaySoundatLocation "/Game/Player/Audio/Sound/1911.1911" (Transformation|GetWorldLocation (Variables|Default|GetMuzzle)) "0, 0, 0" 1.0 1.0 0.1 0 0 0))

(event Custom|Symulate%20PH/Destroy/Collision
  (params (Collision :type ECollisionEnabled%20Enum :default "NoCollision") (bSimulate :type Boolean) (Destroy :type Boolean) (Destroy%20after%2030s :type Boolean))
  (bind _m1911 (Variables|Default|Getm1911))
  (Collision|SetCollisionEnabled _m1911 Collision)
  (if bSimulate
    (Physics|SetSimulatePhysics _m1911 bSimulate)
    (if Destroy%20after%2030s
      (Utilities|FlowControl|Delay 3e+01)))
  (if (or Destroy Destroy%20after%2030s)
    (Actor|DestroyActor)))

(event EventBeginPlay)

(event Collision|EventActorBeginOverlap
  (params (OtherActor :type Actor%20Object%20Reference)))

(event EventTick
  (params (DeltaSeconds :type Float%20%28single-precision%29)))

(fn ConstructionScript)