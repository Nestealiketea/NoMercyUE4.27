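; Base bullet projectile actor that resolves its first impact with surface-dependent damage, effects and sound, then destroys itself.
; On Hit, a small sphere trace at the hit location reads the physical surface type.
; Body-zone and vehicle surfaces apply tiered damage through Character_BP cast from the hit actor, while environment surfaces choose impact particles.
; The selected sound and emitter play at the impact point; a scale timeline with delayed destroy is unconnected.
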(event EventBeginPlay)

(event Collision|EventActorBeginOverlap
  (params (OtherActor :type Actor%20Object%20Reference)))

(event EventTick
  (params (DeltaSeconds :type Float%20%28single-precision%29)))

(event Collision|EventHit
  (params (MyComp :type Primitive%20Component%20Object%20Reference) (Other :type Actor%20Object%20Reference) (OtherComp :type Primitive%20Component%20Object%20Reference) (bSelfMoved :type Boolean) (HitLocation :type Vector :default "0, 0, 0") (HitNormal :type Vector :default "0, 0, 0") (NormalImpulse :type Vector :default "0, 0, 0") (Hit :type Hit%20Result%20Structure%20%28by%20ref%29))
  (Utilities|FlowControl|DoOnce false
    (:Completed
      (bind (_outhit _returnvalue) (Collision|SphereTraceForObjects HitLocation (+ HitLocation "0.000000,0.000000,1.000000") 5.0 (Utilities|Array|MakeArray "ObjectTypeQuery4" "ObjectTypeQuery1") false 0 "None" false))
      (if _returnvalue
        (bind _ascharacter_bp (Utilities|Casting|CastToCharacter_BP Other)
          (:then
            _)
          (:CastFailed
            _))
        (switch Utilities|FlowControl|Switch|SwitchonEPhysicalSurface (Collision|GetSurfaceType _outhit)
          (:SurfaceType_Default
            _)
          (:SurfaceType1
            (Default|ApplyDamageonEnemy _ascharacter_bp (.HitActor (Collision|BreakHitResult _outhit)) (.Time (Collision|BreakHitResult _outhit)) 7e+01)
            (Variables|Default|SetSound "/Game/Player/Audio/Hit/Hit_Body_Cue.Hit_Body_Cue" :!label _label))
          (:SurfaceType2
            (Default|ApplyDamageonEnemy _ascharacter_bp (.HitActor (Collision|BreakHitResult _outhit)) (.Time (Collision|BreakHitResult _outhit)) 4e+01)
            (goto _label))
          (:SurfaceType3
            (Default|ApplyDamageonEnemy _ascharacter_bp (.HitActor (Collision|BreakHitResult _outhit)) (.Time (Collision|BreakHitResult _outhit)) 15.0)
            (goto _label))
          (:SurfaceType4
            (Default|ApplyDamageonEnemy _ascharacter_bp (.HitActor (Collision|BreakHitResult _outhit)) (.Time (Collision|BreakHitResult _outhit)) 5.0)
            (goto _label))
          (:SurfaceType5
            (Variables|Default|SetSound "/Game/Player/Audio/Hit/Hit_Car_Cue.Hit_Car_Cue")
            (Default|ApplyDamageonEnemy _ascharacter_bp (.HitActor (Collision|BreakHitResult _outhit)) (.Time (Collision|BreakHitResult _outhit)) 5e+01))
          (:SurfaceType6
            (Variables|Default|SetSound "/Game/Player/Audio/Hit/Hit_Ground_Cue.Hit_Ground_Cue")
            (Variables|Default|SetEmitter "/Game/Player/Particle/Surface_Emitters/Impuct/Particles/PS_Impact_Dirt.PS_Impact_Dirt"))
          (:SurfaceType7
            (Variables|Default|SetSound "/Game/Player/Audio/Hit/Hit_Ground_Cue.Hit_Ground_Cue")
            (Variables|Default|SetEmitter "/Game/Player/Particle/Surface_Emitters/Impuct/Particles/PS_Impact_Dirt.PS_Impact_Dirt"))
          (:SurfaceType8
            (Variables|Default|SetSound "/Game/Player/Audio/Hit/Hit_Ground_Cue.Hit_Ground_Cue")
            (Variables|Default|SetEmitter "/Game/Player/Particle/Surface_Emitters/Impuct/Particles/PS_Impact_Dirt.PS_Impact_Dirt"))
          (:SurfaceType9
            (Variables|Default|SetSound "/Game/Player/Audio/Hit/Hit_Ground_Cue.Hit_Ground_Cue")
            (Variables|Default|SetEmitter "/Game/Player/Particle/Surface_Emitters/Impuct/Particles/PS_Impact_Concrete.PS_Impact_Concrete"))
          (:SurfaceType10
            (Variables|Default|SetSound "/Game/Player/Audio/Hit/Hit_Ground_Cue.Hit_Ground_Cue")
            (Variables|Default|SetEmitter "/Game/Player/Particle/Surface_Emitters/Impuct/Particles/PS_Impact_Dirt.PS_Impact_Dirt"))
          (:SurfaceType11
            (Variables|Default|SetSound "/Game/Player/Audio/Hit/Hit_Ground_Cue.Hit_Ground_Cue")
            (Variables|Default|SetEmitter "/Game/Player/Particle/Surface_Emitters/Impuct/Particles/PS_Impact_Dirt.PS_Impact_Dirt"))
          (:SurfaceType12
            (Variables|Default|SetSound "/Game/Player/Audio/Hit/Hit_Ground_Cue.Hit_Ground_Cue")
            (Variables|Default|SetEmitter "/Game/Player/Particle/Surface_Emitters/Impuct/Particles/PS_Impact_Water.PS_Impact_Water"))
          (:SurfaceType13
            (Variables|Default|SetSound "/Game/Player/Audio/Hit/Hit_Wood_Cue.Hit_Wood_Cue")
            (Variables|Default|SetEmitter "/Game/Player/Particle/Surface_Emitters/Impuct/Particles/PS_Impact_Wood.PS_Impact_Wood"))
          (:SurfaceType14
            (Variables|Default|SetSound "/Game/Player/Audio/Hit/Hit_Ground_Cue.Hit_Ground_Cue")
            (Variables|Default|SetEmitter "/Game/Player/Particle/Surface_Emitters/Impuct/Particles/PS_Impact_Dirt.PS_Impact_Dirt"))))
      (Effects|SpawnEmitteratLocation (Variables|Default|GetEmitter) (.ImpactPoint (Collision|BreakHitResult _outhit)) (Math|Rotator|MakeRotfromZ (.Normal (Collision|BreakHitResult _outhit))) "3.000000,3.000000,3.000000")
      (Audio|PlaySoundatLocation (Variables|Default|GetSound) (.ImpactPoint (Collision|BreakHitResult _outhit)) "0, 0, 0" 1.0 1.0 0.0 0 0 0)
      (Actor|DestroyActor))))

(fn ConstructionScript)